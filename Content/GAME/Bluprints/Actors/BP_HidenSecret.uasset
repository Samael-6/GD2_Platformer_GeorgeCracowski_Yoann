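; BP_HidenSecret is an interactable actor with a plane and text render that toggles a secret message display.
; BeginPlay caches the plane's original material and sets up two message strings.
; Each Interact event flip-flops between a black material with a hint-style text and the original material with the secret text.
; Actor overlap begin and end show and hide an "E interact" prompt through BPCInteract.
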(event `self.ReceiveBeginPlay`
  (set `self.DefaultMaterial` (`PrimitiveComponent.GetMaterial` (`self.Plane`) 0))
  (set `self.Message` "It's a secret")
  (set `self.MessageTemp` "You know how interact"))

(event `/Game/GAME/Bluprints/BPI/BPI_Interact.Interact`
  (`/Engine/EditorBlueprintResources/StandardMacros.FlipFlop`
    (:`A`
      (`PrimitiveComponent.SetMaterial` (`self.Plane`) 0 "/Game/StarterContent/Blueprints/Assets/M_LightStage_Skybox_Black.M_LightStage_Skybox_Black")
      (`TextRenderComponent.K2_SetText` (`self.TextRender`) (`self.MessageTemp`)))
    (:`B`
      (`PrimitiveComponent.SetMaterial` (`self.Plane`) 0 (`self.DefaultMaterial`))
      (`TextRenderComponent.K2_SetText` (`self.TextRender`) (`self.Message`)))))

(event `self.ReceiveActorBeginOverlap`
  (params (OtherActor :type "Actor Object Reference"))
  (bind _bpc_interact (`self.BPC_Interact`))
  (set `/Game/GAME/Bluprints/BPC/BPC_Interact.TxtInteract` "E interact" _bpc_interact)
  (`/Game/GAME/Bluprints/BPC/BPC_Interact.ShowText` _bpc_interact))

(event `self.ReceiveActorEndOverlap`
  (params (OtherActor :type "Actor Object Reference"))
  (`/Game/GAME/Bluprints/BPC/BPC_Interact.UnshowText` (`self.BPC_Interact`)))

(fn `UserConstructionScript`)
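; BP_PlatformeUpDown is an interactable platform actor that requires battery power, tracked by IsPower on BP_GameInstance.
; On overlap, its BPCInteract component shows "Press E" or "No Battery" depending on that flag, and hides the text when overlap ends.
; Pressing E while powered reveals BPBattery and sets IsMoving; the handler has no overlap check, and the graph contains no movement logic.
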(event `self.ReceiveBeginPlay`
  (bind _asbp_game_instance (cast `/Game/GAME/Bluprints/BP_GameInstance` (`GameplayStatics.GetGameInstance`)))
  (set `self.Ref_BP_GameInstance` _asbp_game_instance))

(event `self.ReceiveActorBeginOverlap`
  (params (OtherActor :type "Actor Object Reference"))
  (bind _bpc_interact (`self.BPC_Interact`))
  (bind _bpc_interact_2 (`self.BPC_Interact`))
  (if (`/Game/GAME/Bluprints/BP_GameInstance.Is_Power` (`self.Ref_BP_GameInstance`))
    (set `/Game/GAME/Bluprints/BPC/BPC_Interact.TxtInteract` "Press E" _bpc_interact_2)
    (`/Game/GAME/Bluprints/BPC/BPC_Interact.ShowText` _bpc_interact_2)
    (else
      (set `/Game/GAME/Bluprints/BPC/BPC_Interact.TxtInteract` "No Battery" _bpc_interact)
      (`/Game/GAME/Bluprints/BPC/BPC_Interact.ShowText` _bpc_interact))))

(event `self.ReceiveActorEndOverlap`
  (params (OtherActor :type "Actor Object Reference"))
  (`/Game/GAME/Bluprints/BPC/BPC_Interact.UnshowText` (`self.BPC_Interact`)))

(event `Key|E`
  (params (Key :type "Key Structure"))
  (:`Pressed`
    (if (`/Game/GAME/Bluprints/BP_GameInstance.Is_Power` (`self.Ref_BP_GameInstance`))
      (`SceneComponent.SetVisibility` (`self.BP_Battery`) true false)
      (set `self.Is_Moving` true))))

(fn `UserConstructionScript`)
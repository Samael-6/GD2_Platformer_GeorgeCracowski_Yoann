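; BP_Key is a key pickup actor that the player collects through an Interact event.
; On BeginPlay it caches the game instance and the player pawn.
; Overlap shows or hides a "Press E" prompt through its BPCInteract component, without filtering the overlapping actor.
; Interacting sets IsOpen and increments the Key count on the game instance, refreshes the player's HUD score, then destroys the key.
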(event `self.ReceiveBeginPlay`
  (bind _asbp_game_instance (cast `/Game/GAME/Bluprints/BP_GameInstance` (`GameplayStatics.GetGameInstance`)))
  (set `self.Ref_BP_GameInstance` _asbp_game_instance)
  (bind _asbp_joueur (cast `/Game/GAME/Bluprints/Actors/BP_Joueur` (`GameplayStatics.GetPlayerPawn` 0)))
  (set `self.Ref_BPJoueur` _asbp_joueur))

(event `/Game/GAME/Bluprints/BPI/BPI_Interact.Interact`
  (bind _ref_bp_gameinstance (`self.Ref_BP_GameInstance`))
  (set `/Game/GAME/Bluprints/BP_GameInstance.Is_Open` true _ref_bp_gameinstance)
  (bind _result (`/Engine/EditorBlueprintResources/StandardMacros.IncrementInt` (`/Game/GAME/Bluprints/BP_GameInstance.Key` _ref_bp_gameinstance))
    (:`  `
      (set `/Game/GAME/Bluprints/BP_GameInstance.Key` _result _ref_bp_gameinstance)
      (`/Game/GAME/Bluprints/Widget/BPW_MainHUD.UpdateScore` (`/Game/GAME/Bluprints/Actors/BP_Joueur.Ref_BPW_MainHUD` (`self.Ref_BPJoueur`)))
      (`self.K2_DestroyActor`))))

(event `self.ReceiveActorBeginOverlap`
  (params (OtherActor :type "Actor Object Reference"))
  (bind _bpc_interact (`self.BPC_Interact`))
  (set `/Game/GAME/Bluprints/BPC/BPC_Interact.TxtInteract` "Press E" _bpc_interact)
  (`/Game/GAME/Bluprints/BPC/BPC_Interact.ShowText` _bpc_interact))

(event `self.ReceiveActorEndOverlap`
  (params (OtherActor :type "Actor Object Reference"))
  (`/Game/GAME/Bluprints/BPC/BPC_Interact.UnshowText` (`self.BPC_Interact`)))

(fn `UserConstructionScript`)
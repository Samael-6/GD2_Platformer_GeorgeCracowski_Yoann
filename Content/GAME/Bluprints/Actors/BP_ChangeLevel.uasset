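; BP_ChangeLevel is an interactable actor that switches the game between Level2 and ThirdPersonMap.
; Its Interact event checks the current level name, opening ThirdPersonMap from Level2 and Level2 from any other level.
; Begin and end overlap show and hide a "Swap Level" prompt through BPCInteract, without filtering which actor overlaps.
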(event `/Game/GAME/Bluprints/BPI/BPI_Interact.Interact`
  (bind _returnvalue (`GameplayStatics.GetCurrentLevelName` true))
  (if (`KismetStringLibrary.EqualEqual_StrStr` _returnvalue "Level2")
    (`GameplayStatics.OpenLevel` "ThirdPersonMap")
    (else
      (`GameplayStatics.OpenLevel` "Level2"))))

(event `self.ReceiveActorBeginOverlap`
  (params (OtherActor :type "Actor Object Reference"))
  (bind _bpc_interact (`self.BPC_Interact`))
  (set `/Game/GAME/Bluprints/BPC/BPC_Interact.TxtInteract` "Swap Level" _bpc_interact)
  (`/Game/GAME/Bluprints/BPC/BPC_Interact.ShowText` _bpc_interact))

(event `self.ReceiveActorEndOverlap`
  (params (OtherActor :type "Actor Object Reference"))
  (`/Game/GAME/Bluprints/BPC/BPC_Interact.UnshowText` (`self.BPC_Interact`)))

(fn `UserConstructionScript`)
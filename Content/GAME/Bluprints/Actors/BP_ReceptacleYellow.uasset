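; BP_ReceptacleYellow is an interactable receptacle that takes a yellow button and removes the BP_BarrierYellow actor found at BeginPlay.
; Overlap shows a BPCInteract prompt based on the GameInstance's yellow-button flag, and end overlap hides it.
; The first Interact reveals FakeButton and marks the receptacle repaired, and the next destroys the barrier once.
; Interact itself does not check whether the button was collected.
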(event `self.ReceiveBeginPlay`
  (bind _asbp_game_instance (cast `/Game/GAME/Bluprints/BP_GameInstance` (`GameplayStatics.GetGameInstance`)))
  (set `self.Ref_GameInstance` _asbp_game_instance)
  (bind _returnvalue (`GameplayStatics.GetActorOfClass` "/Game/GAME/Bluprints/Actors/BP_BarrierYellow.BP_BarrierYellow_C"))
  (set `self.Ref_BerrierYellow` _returnvalue))

(event `self.ReceiveActorBeginOverlap`
  (params (OtherActor :type "Actor Object Reference"))
  (if (`/Game/GAME/Bluprints/BP_GameInstance.Is_YellowButtonCollect` (`self.Ref_GameInstance`))
    (if (not (`self.Is_destroy`))
      (set `/Game/GAME/Bluprints/BPC/BPC_Interact.TxtInteract` "E press button" (`self.BPC_Interact`))
      (`/Game/GAME/Bluprints/BPC/BPC_Interact.ShowText` (`self.BPC_Interact`) :!label _label))
    (else
      (set `/Game/GAME/Bluprints/BPC/BPC_Interact.TxtInteract` "You need a button" (`self.BPC_Interact`))
      (goto _label))))

(event `self.ReceiveActorEndOverlap`
  (params (OtherActor :type "Actor Object Reference"))
  (`/Game/GAME/Bluprints/BPC/BPC_Interact.UnshowText` (`self.BPC_Interact`)))

(event `/Game/GAME/Bluprints/BPI/BPI_Interact.Interact`
  (if (`self.Is_Repared`)
    (if (not (`self.Is_destroy`))
      (`self.K2_DestroyActor` (`self.Ref_BerrierYellow`))
      (set `self.Is_destroy` true)
      (`/Game/GAME/Bluprints/BPC/BPC_Interact.UnshowText` (`self.BPC_Interact`)))
    (else
      (`SceneComponent.SetVisibility` (`self.FakeButton`) true false)
      (set `self.Is_Repared` true))))

(fn `UserConstructionScript`)
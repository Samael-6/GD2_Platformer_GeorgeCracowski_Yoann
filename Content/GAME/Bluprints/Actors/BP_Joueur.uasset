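; BP_Joueur is the player actor Blueprint, handling item collection, interaction and the main HUD.
; BeginPlay creates BPW_MainHUD and adds it to the viewport.
; On overlap, actors with a collectible component go to the collect component and refresh the HUD score; otherwise, BPI_Interact implementers are stored as the active target.
; IA_Interact sends that target InteractMessage while interaction is enabled, and end overlap clears the flag.
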(event `self.ReceiveBeginPlay`
  (`parent.ReceiveBeginPlay`)
  (bind _returnvalue (`|CreateWidget` "/Game/GAME/Bluprints/Widget/BPW_MainHUD.BPW_MainHUD_C"))
  (bind _output_get (set `self.Ref_BPW_MainHUD` _returnvalue))
  (`UserWidget.AddToViewport` _output_get 0))

(event `self.ReceiveActorBeginOverlap`
  (params (OtherActor :type "Actor Object Reference"))
  (bind _returnvalue (`self.GetComponentByClass` OtherActor "/Game/GAME/Bluprints/BPC/BPC_CollectibleComponent.BPC_CollectibleComponent_C"))
  (`/Engine/EditorBlueprintResources/StandardMacros.IsValid` _returnvalue
    (:`Is Valid`
      (`/Game/GAME/Bluprints/BPC/BPC_CollectComponent.Collect` (`self.BPC_CollectComponent`) _returnvalue)
      (`/Game/GAME/Bluprints/Widget/BPW_MainHUD.UpdateScore` (`self.Ref_BPW_MainHUD`)))
    (:`Is Not Valid`
      (if (`KismetSystemLibrary.DoesImplementInterface` OtherActor "/Game/GAME/Bluprints/BPI/BPI_Interact.BPI_Interact_C")
        (set `self.Other Actor` OtherActor)
        (set `self.Is_Activable` true)))))

(event `self.ReceiveActorEndOverlap`
  (params (OtherActor :type "Actor Object Reference"))
  (if (== OtherActor (`self.Other Actor`))
    (set `self.Is_Activable` false)))

(event `EnhancedInput|/Game/ThirdPerson/Input/Actions/IA_Interact`
  (params (ActionValue :type Boolean) (ElapsedSeconds :type "Float (double-precision)") (TriggeredSeconds :type "Float (double-precision)") (InputAction :type "InputAction Object Reference" :default "/Game/ThirdPerson/Input/Actions/IA_Interact.IA_Interact"))
  (:`Started`
    (if (`self.Is_Activable`)
      (message `/Game/GAME/Bluprints/BPI/BPI_Interact.Interact` (`self.Other Actor`)))))

(fn `UserConstructionScript`
  (`parent.UserConstructionScript`))
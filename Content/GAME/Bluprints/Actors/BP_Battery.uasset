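; BP_Battery is a collectible battery actor that turns on a power flag when picked up.
; On BeginPlay it caches BP_GameInstance, and its Interact event sets IsPower there before destroying the actor.
; Actor overlap drives the BPCInteract component, showing a collect prompt on entry and hiding it on exit.
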(event `self.ReceiveBeginPlay`
  (bind _asbp_game_instance (cast `/Game/GAME/Bluprints/BP_GameInstance` (`GameplayStatics.GetGameInstance`)))
  (set `self.Ref_GameInstance` _asbp_game_instance))

(event `/Game/GAME/Bluprints/BPI/BPI_Interact.Interact`
  (set `/Game/GAME/Bluprints/BP_GameInstance.Is_Power` true (`self.Ref_GameInstance`))
  (`self.K2_DestroyActor`))

(event `self.ReceiveActorBeginOverlap`
  (params (OtherActor :type "Actor Object Reference"))
  (bind _bpc_interact (`self.BPC_Interact`))
  (set `/Game/GAME/Bluprints/BPC/BPC_Interact.TxtInteract` "E collect" _bpc_interact)
  (`/Game/GAME/Bluprints/BPC/BPC_Interact.ShowText` _bpc_interact))

(event `self.ReceiveActorEndOverlap`
  (params (OtherActor :type "Actor Object Reference"))
  (`/Game/GAME/Bluprints/BPC/BPC_Interact.UnshowText` (`self.BPC_Interact`)))

(fn `UserConstructionScript`)
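; BPC_Interact is an interaction component that shows and hides an on-screen text prompt.
; On BeginPlay it creates a BPW_Interact widget and keeps a reference to it.
; ShowText copies its TxtInteract value into the widget and adds it to the viewport, while UnshowText removes the widget, so the same instance is reused for each prompt.
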(event `self.ReceiveBeginPlay`
  (bind _returnvalue (`|CreateWidget` "/Game/GAME/Bluprints/Widget/BPW_Interact.BPW_Interact_C"))
  (set `self.Ref_BPW_Interact` _returnvalue))

(fn `ShowText`
  (bind _ref_bpw_interact (`self.Ref_BPW_Interact`))
  (set `TextBlock.Text` (`self.TxtInteract`) (`/Game/GAME/Bluprints/Widget/BPW_Interact.Txt_Interact` _ref_bpw_interact))
  (`UserWidget.AddToViewport` _ref_bpw_interact 0))

(fn `UnshowText`
  (`Widget.RemoveFromParent` (`self.Ref_BPW_Interact`)))
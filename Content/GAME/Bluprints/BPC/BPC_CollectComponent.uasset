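; BPC_CollectComponent is an actor component that handles picking up collectibles and adding their value to the game score.
; On BeginPlay it caches the BP_GameInstance.
; Its Collect function adds the collectible component's Value to the Score on that game instance, then destroys the collectible if it is flagged IsDestroyable.
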(event `self.ReceiveBeginPlay`
  (bind _asbp_game_instance (cast `/Game/GAME/Bluprints/BP_GameInstance` (`GameplayStatics.GetGameInstance`)))
  (set `self.V_GameInstance` _asbp_game_instance))

(fn `Collect`
  (params (component :type "/Game/GAME/Bluprints/BPC/BPC_CollectibleComponent Object Reference"))
  (bind _v_gameinstance (`self.V_GameInstance`))
  (set `/Game/GAME/Bluprints/BP_GameInstance.Score` (+ (`/Game/GAME/Bluprints/BPC/BPC_CollectibleComponent.Value` component) (`/Game/GAME/Bluprints/BP_GameInstance.Score` _v_gameinstance)) _v_gameinstance)
  (if (`/Game/GAME/Bluprints/BPC/BPC_CollectibleComponent.IsDestroyable` component)
    (`/Game/GAME/Bluprints/BPC/BPC_CollectibleComponent.Destroy_BP_Collectible` component)))